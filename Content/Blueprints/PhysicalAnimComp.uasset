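; Component that adds partial physical animation to the BP_Gorby character.
; On BeginPlay it adds a PhysicalAnimationComponent to its owner, caches Gorby's mesh and movement component, and binds the mesh to it.
; Every Tick it re-enables physics simulation from bone_014 downward, then applies the "None" physical animation profile to the bodies below that bone, excluding it.
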(event `self.ReceiveBeginPlay`
  (bind _returnvalue (`|AddComponentByClass` (`self.GetOwner`) "/Script/Engine.PhysicalAnimationComponent"))
  (bind _output_get (set `self.PhysicalAnimationComponent` _returnvalue))
  (bind _asbp_gorby (cast `/Game/Blueprints/BP_Gorby` (`self.GetOwner`)))
  (bind _output_get_2 (set `self.As Gorby` _asbp_gorby))
  (set `self.Character Movement` (`Character.CharacterMovement` _output_get_2))
  (bind _output_get_3 (set `self.Mesh` (`Character.Mesh` _output_get_2)))
  (`PhysicalAnimationComponent.SetSkeletalMeshComponent` _output_get _output_get_3))

(event `self.ReceiveTick`
  (params (DeltaSeconds :type "Float (single-precision)"))
  (`SkeletalMeshComponent.SetAllBodiesBelowSimulatePhysics` (`self.Mesh`) "bone_014" true true)
  (`PhysicalAnimationComponent.ApplyPhysicalAnimationProfileBelow` (`self.PhysicalAnimationComponent`) "bone_014" "None" false false))
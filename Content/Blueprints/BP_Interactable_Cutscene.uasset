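; Interactable Blueprint that plays a Level Sequence cutscene and completes a mission when the player interacts with it.
; BeginPlay creates a player for LevelSequenceToPlay, but only if LevelSequenceComponent is already valid, and stores it in that same variable.
; OnInteract fires once, plays that sequence if valid, then immediately calls CompleteMission with MissionNumber on the level's MissionManager without waiting for playback to end.
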(event `/Game/Blueprints/BPI_Interactable.OnInteract`
  (`/Engine/EditorBlueprintResources/StandardMacros.DoOnce` false
    (:`Completed`
      (`self.Level Sequence Component`
        (:`then`
          (`MovieSceneSequencePlayer.Play` (`self.Level Sequence Component`)))
        (:`else`
          _))
      (bind _returnvalue (`GameplayStatics.GetActorOfClass` "/Game/Blueprints/MissionManager.MissionManager_C"))
      (`/Game/Blueprints/MissionManager.CompleteMission` _returnvalue (`self.MissionNumber`)))))

(event `self.ReceiveBeginPlay`
  (`self.Level Sequence Component`
    (:`then`
      (bind (_outactor _returnvalue) (`LevelSequencePlayer.CreateLevelSequencePlayer` (`self.Level Sequence To Play`)))
      (set `self.Level Sequence Component` _returnvalue))
    (:`else`)))

(fn `UserConstructionScript`)
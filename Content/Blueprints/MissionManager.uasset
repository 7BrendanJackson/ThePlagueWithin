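; MissionManager tracks completion of three missions and shows them through a Missions widget.
; On BeginPlay it creates the Missions widget and adds it to the viewport.
; CompleteMission uses a per-task flag so each mission number notifies the widget only the first time it completes.
; The Strike event completes mission 1.
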(event `self.ReceiveBeginPlay`
  (bind _returnvalue (`|CreateWidget` "/Game/Blueprints/Missions.Missions_C"))
  (set `self.Widget` _returnvalue)
  (`UserWidget.AddToViewport` _returnvalue 0))

(event `Strike`
  (`self.CompleteMission` 1))

(fn `CompleteMission`
  (params (MissionNumber :type Integer))
  (switch `int` MissionNumber
    (:`1`
      (if (not (`self.Task1`))
        (set `self.Task1` true)
        (`/Game/Blueprints/Missions.CompleteMission` (`self.Widget`) MissionNumber :!label _label)))
    (:`2`
      (if (not (`self.Task2`))
        (set `self.Task2` true)
        (goto _label)))
    (:`3`
      (if (not (`self.Task3`))
        (set `self.Task3` true)
        (goto _label)))))

(fn `UserConstructionScript`)
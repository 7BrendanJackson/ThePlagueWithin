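; BP_StuckRat is an interactable trapped rat that the player frees once.
; On interact, it tells the child-actor BP_RAT_NPC to run GOTO and play its freedom reaction.
; A timeline then scales the trap mesh by its Shrink curve and destroys the trap component when it finishes.
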(event `/Game/Blueprints/BPI_Interactable.OnInteract`
  (`/Engine/EditorBlueprintResources/StandardMacros.DoOnce` false
    (:`Completed`
      (bind _asbp_rat_npc (cast `/Game/Blueprints/BP_RAT_NPC` (`ChildActorComponent.ChildActor` (`self.NPC`))))
      (`/Game/Blueprints/BP_RAT_NPC.GOTO` _asbp_rat_npc)
      (`/Game/Blueprints/BP_RAT_NPC.PlayFreedom` _asbp_rat_npc)
      (bind (_direction _shrink) (`Timeline|Timeline` :!via `PlayFromStart`)
        (:`Update`
          (`SceneComponent.SetWorldScale3D` (`self.Trap`) (`KismetMathLibrary.Conv_DoubleToVector` _shrink)))
        (:`Finished`
          (`ActorComponent.K2_DestroyComponent` (`self.Trap`)))))))

(fn `UserConstructionScript`)
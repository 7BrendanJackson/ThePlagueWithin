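; Test interactable actor that plays a configurable level sequence as a cutscene, once, when interacted with.
; BeginPlay creates and stores the sequence player, and OnInteract plays it through a DoOnce with a debug print.
; Entering the Sphere trigger adds a cutscene prompt widget to the viewport.
; Leaving it calls RemoveAllWidgets, clearing every viewport widget rather than only the prompt.
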(event `/Game/Blueprints/BPI_Interactable.OnInteract`
  (`/Engine/EditorBlueprintResources/StandardMacros.DoOnce` false
    (:`Completed`
      (`KismetSystemLibrary.PrintString` "Interacted with")
      (`MovieSceneSequencePlayer.Play` (`self.Level Sequence Component`)))))

(event `self.ReceiveBeginPlay`
  (bind (_outactor _returnvalue) (`LevelSequencePlayer.CreateLevelSequencePlayer` (`self.Level Sequence To Play`)))
  (set `self.Level Sequence Component` _returnvalue))

(event `self.Sphere.OnComponentBeginOverlap`
  (params (OverlappedComponent :type "PrimitiveComponent Object Reference") (OtherActor :type "Actor Object Reference") (OtherComp :type "PrimitiveComponent Object Reference") (OtherBodyIndex :type Integer) (bFromSweep :type Boolean) (SweepResult :type "HitResult Structure (by ref)"))
  (bind _returnvalue (`|CreateWidget` "/Game/Blueprints/Cutscenes/W_CutscenePrompt.W_CutscenePrompt_C"))
  (`UserWidget.AddToViewport` _returnvalue 0))

(event `self.Sphere.OnComponentEndOverlap`
  (params (OverlappedComponent :type "PrimitiveComponent Object Reference") (OtherActor :type "Actor Object Reference") (OtherComp :type "PrimitiveComponent Object Reference") (OtherBodyIndex :type Integer))
  (`WidgetLayoutLibrary.RemoveAllWidgets`))

(fn `UserConstructionScript`)
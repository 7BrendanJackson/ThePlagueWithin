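; Rat NPC that, when its Roaming flag is set, wanders between random reachable navmesh points around itself from BeginPlay.
; A delayed polling loop checks movement velocity and issues a new move whenever the rat has slowed or stopped.
; On each repick there is a small random chance to play its audio through PlayFreedom.
; ReportPosition returns the actor location, while ReportVelocity only returns a zero vector.
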(event `PlayFreedom`
  (`AudioComponent.Play` (`self.Audio`) 0.0))

(event `GOTO`
  (`AIBlueprintHelperLibrary.SimpleMoveToLocation` (`self.GetController`) (`NavigationSystemV1.K2_GetRandomReachablePointInRadius` (`self.K2_GetActorLocation`) 5000.0 null null) :!label _label)
  (`KismetSystemLibrary.Delay` 2.0 :!label _label_2)
  (if (> (`KismetMathLibrary.VSize` (`MovementComponent.Velocity` (`self.CharacterMovement`))) 100.0)
    (goto _label_2)
    (elif (>= (`KismetMathLibrary.RandomFloat`) 0.95)
      (`self.PlayFreedom`)
      (goto _label)
      (else
        (goto _label)))))

(event `self.ReceiveBeginPlay`
  (if (`self.Roaming?`)
    (goto _label)))

(fn `ReportPosition`
  (returns (Location :type "Vector Structure"))
  (return (`self.K2_GetActorLocation`)))

(fn `ReportVelocity`
  (returns (Velocity :type "Vector2D Structure"))
  (return (0.0 0.0)))

(fn `UserConstructionScript`)
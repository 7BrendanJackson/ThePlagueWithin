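; Main menu controller that turns Enhanced Input navigate and confirm actions into button hover and presses.
; BeginPlay collects BP_Menu3D actors except "Title", adds the menu mapping context and caches the main menu and credits widgets.
; Navigation steps a clamped per-layer button index; confirm plays a sound and opens the Cutscene level, shows credits or quits, or backs out on the credits layer.
; Tick prints layer and button debug text.
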(event `self.ReceiveBeginPlay`
  (bind _menulayers (`self.MenuLayers`))
  (`|ExecutionSequence`
    (:`then_0`
      (bind _outactors (`GameplayStatics.GetAllActorsOfClass` "/Game/Blueprints/MenuBlueprints/BP_Menu3D.BP_Menu3D_C"))
      (`|VariableSetRef` _menulayers _outactors)
      (for (_array_element _array_index) _menulayers
        (if (== (`KismetSystemLibrary.GetDisplayName` _array_element) "Title")
          (`KismetArrayLibrary.Array_Remove` (`self.MenuLayers`) _array_index))))
    (:`then_1`
      (bind _asplayer_controller (cast `PlayerController` (`self.GetController`)))
      (message `EnhancedInputSubsystemInterface.AddMappingContext` (pcsubsystem `EnhancedInputLocalPlayerSubsystem` _asplayer_controller) "/Game/ThirdPerson/Input/IMC_Menu.IMC_Menu" 0 (struct))
      (bind _foundwidgets (`WidgetBlueprintLibrary.GetAllWidgetsOfClass` "/Game/Blueprints/MenuBlueprints/W_MainMenuu.W_MainMenuu_C" false))
      (set `self.MenuWidget` (`|GetArrayItem` _foundwidgets))
      (bind _foundwidgets_2 (`WidgetBlueprintLibrary.GetAllWidgetsOfClass` "/Game/Blueprints/MenuBlueprints/W_Creditss.W_Creditss_C" false))
      (set `self.CreditsWidget` (`|GetArrayItem` _foundwidgets_2))
      (`KismetSystemLibrary.Delay` 0.2)
      (`/Game/Blueprints/MenuBlueprints/W_MainMenuu.CallOnHover` (`self.MenuWidget`) (`|GetArrayItem` (`self.CurrentButton`) (`self.CurrentLayer`)) :!label _label)
      (if (== (`self.CurrentLayer`) 1)
        _))))

(event `EnhancedInput|/Game/ThirdPerson/Input/IA_MenuNavigate`
  (params (ActionValue :type "Float (double-precision)") (ElapsedSeconds :type "Float (double-precision)") (TriggeredSeconds :type "Float (double-precision)") (InputAction :type "InputAction Object Reference" :default "/Game/ThirdPerson/Input/IA_MenuNavigate.IA_MenuNavigate"))
  (bind _currentlayer (`self.CurrentLayer`))
  (bind _currentbutton (`self.CurrentButton`))
  (:`Triggered`
    (`KismetArrayLibrary.Array_Set` _currentbutton _currentlayer (`KismetMathLibrary.Clamp` (+ (`|GetArrayItem` _currentbutton _currentlayer) (`KismetMathLibrary.SelectInt` 1 -1 (> ActionValue 0.0))) 0 (`|GetArrayItem` (`self.Max`) (`self.CurrentLayer`))))
    (goto _label)))

(event `EnhancedInput|/Game/ThirdPerson/Input/IA_MenuConfirm`
  (params (ActionValue :type Boolean) (ElapsedSeconds :type "Float (double-precision)") (TriggeredSeconds :type "Float (double-precision)") (InputAction :type "InputAction Object Reference" :default "/Game/ThirdPerson/Input/IA_MenuConfirm.IA_MenuConfirm"))
  (bind _creditswidget (`self.CreditsWidget`))
  (bind _currentlayer (`self.CurrentLayer`))
  (:`Triggered`
    (if (== _currentlayer 1)
      (`/Game/Blueprints/MenuBlueprints/W_Creditss.PressBack` _creditswidget)
      (`/Game/Blueprints/MenuBlueprints/W_Creditss.Unhover` _creditswidget)
      (goto _label)
      (else
        (switch `int` (`|GetArrayItem` (`self.CurrentButton`) _currentlayer)
          (:`0`
            (`self.PressPlay`))
          (:`1`
            (`/Game/Blueprints/MenuBlueprints/W_MainMenuu.PressCredits` (`self.MenuWidget`))
            (`/Game/Blueprints/MenuBlueprints/W_Creditss.Hover` _creditswidget))
          (:`2`
            (`/Game/Blueprints/MenuBlueprints/W_MainMenuu.PressQuit` (`self.MenuWidget`))))))))

(event `self.ReceiveTick`
  (params (DeltaSeconds :type "Float (single-precision)"))
  (`KismetSystemLibrary.PrintString` (`KismetStringLibrary.BuildString_Int` "Layer: " "" (`self.CurrentLayer`)) true true (struct :`G` 0.66 :`B` 1.0 :`A` 1.0) 2.0 "Nonsssse")
  (`KismetSystemLibrary.PrintString` (`KismetStringLibrary.BuildString_Int` "Button:" "" (`|GetArrayItem` (`self.CurrentButton`))) true true (struct :`G` 0.66 :`B` 1.0 :`A` 1.0) 2.0 "sasa"))

(fn `Hover`
  (params (Layer :type Integer) (Button :type Integer)))

(fn `PressPlay`
  (`GameplayStatics.PlaySound2D` null 1.0 1.0 0.0 null null)
  (`GameplayStatics.OpenLevelBySoftObjectPtr` "/Game/ThirdPerson/Maps/Cutscene.Cutscene"))

(fn `UserConstructionScript`)
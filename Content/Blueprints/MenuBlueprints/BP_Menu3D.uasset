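; BP_Menu3D is an actor that presents a menu widget in the world and moves the player's view to linked menus.
; On BeginPlay it binds to the TransitionToLinkedMenu dispatcher on its W_MainMenu3D widget, whose index selects an entry in LinkedMenus.
; A transition disables its own collision, enables the target's, and blends the view target to that menu with an eased, outgoing-locked blend.
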(event `self.ReceiveBeginPlay`
  (bind _asw_main_menu_3d (cast `/Game/Blueprints/MenuBlueprints/W_MainMenu3D` (`WidgetComponent.GetUserWidgetObject` (`self.Widget`))))
  (add `/Game/Blueprints/MenuBlueprints/W_MainMenu3D.TransitionToLinkedMenu` _asw_main_menu_3d (delegate `OnTransitionBetweenMenus`)))

(event `OnTransitionBetweenMenus`
  (params (MenuIndex :type Integer))
  (if (`KismetArrayLibrary.Array_IsValidIndex` (`self.LinkedMenus`) MenuIndex)
    (`self.TransitionTo` (`|GetArrayItem` (`self.LinkedMenus`) MenuIndex))))

(event `TransitionTo`
  (params (`New Menu` :type "/Game/Blueprints/MenuBlueprints/BP_Menu3D Object Reference"))
  (`self.SetActorEnableCollision` false)
  (`self.SetActorEnableCollision` `New Menu` true)
  (`PlayerController.SetViewTargetWithBlend` (`GameplayStatics.GetPlayerController` 0) `New Menu` 2.0 "VTBlend_EaseInOut" 2.0 true))

(fn `UserConstructionScript`)
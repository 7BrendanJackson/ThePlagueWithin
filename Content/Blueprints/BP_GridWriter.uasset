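; Grid writer actor that feeds the positions and velocities of tracked actors into a Niagara grid system.
; On BeginPlay it gathers BPI_GridReporter actors, stores the first as Player, and registers itself as the system's data receiver.
; Each tick it queries them through the interface and pushes location-plus-radius Vector4 and normalized 2D velocity arrays into Niagara user parameters.
; The ParticleData callback only prints a confirmation on first receipt.
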(event `self.ReceiveBeginPlay`
  (bind _returnvalue (`KismetArrayLibrary.Array_Length` (`self.ActorsToTrack`)))
  (`|ExecutionSequence`
    (:`then_0`
      (bind _outactors (`GameplayStatics.GetAllActorsWithInterface` "/Game/Blueprints/BPI_GridReporter.BPI_GridReporter_C"))
      (for _array_element _outactors
        (if (`KismetSystemLibrary.DoesImplementInterface` _array_element "/Game/Blueprints/BPI_GridReporter.BPI_GridReporter_C")
          (`KismetArrayLibrary.Array_Add` (`self.ActorsToTrack`) _array_element)
          (set `self.Player` _array_element)
          (break)))
      (for _array_element_2 _outactors
        (`KismetArrayLibrary.Array_AddUnique` (`self.ActorsToTrack`) _array_element_2))
      (`KismetArrayLibrary.Array_Resize` (`self.ActorLocations`) _returnvalue)
      (`KismetArrayLibrary.Array_Resize` (`self.ActorVelocity`) _returnvalue))
    (:`then_1`
      (`NiagaraComponent.SetVariableObject` (`self.NiagaraGrid`) "User.Receiver" self))))

(event `self.ReceiveTick`
  (params (DeltaSeconds :type "Float (single-precision)"))
  (bind _niagaragrid (`self.NiagaraGrid`))
  (for (_array_element _array_index) (`self.ActorsToTrack`)
    (`/Engine/EditorBlueprintResources/StandardMacros.IsValid` _array_element
      (:`Is Valid`
        (bind _location (message `/Game/Blueprints/BPI_GridReporter.ReportPosition` _array_element))
        (`KismetArrayLibrary.Array_Set` (`self.ActorLocations`) _array_index (`KismetMathLibrary.MakeVector4` (.x _location) (.y _location) (.z _location) (`self.Radius`)))
        (bind _velocity (message `/Game/Blueprints/BPI_GridReporter.ReportVelocity` _array_element))
        (`KismetArrayLibrary.Array_Set` (`self.ActorVelocity`) _array_index (`KismetMathLibrary.Normal2D` _velocity)))))
  (`NiagaraDataInterfaceArrayFunctionLibrary.SetNiagaraArrayVector4` _niagaragrid "User.Locations" (`self.ActorLocations`))
  (`NiagaraDataInterfaceArrayFunctionLibrary.SetNiagaraArrayVector2D` _niagaragrid "User.Velocity" (`self.ActorVelocity`)))

(event `self.ReceiveParticleData`
  (params (Data :type "Array of BasicParticleData Structure (by ref)") (NiagaraSystem :type "NiagaraSystem Object Reference") (SimulationPositionOffset :type "Vector Structure (by ref)"))
  (if (not (`self.Data Receieved`))
    (`KismetSystemLibrary.PrintString` "Data Received")
    (set `self.Data Receieved` true)))

(fn `UserConstructionScript`)